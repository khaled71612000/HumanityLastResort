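; BP_Hotel is a hotel building actor that shows its name and a cash amount through two UI widget components.
; On BeginPlay it creates a name widget from NameView and a cash widget, then assigns each to its component.
; A custom event adds incoming cash to the widget's running amount, coloring it green for positive changes and red otherwise.
; GetName is a stub returning an empty string.
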(event `self.ReceiveBeginPlay`
  (bind _returnvalue (`|CreateWidget` "/Game/UI/WBP_ShowName.WBP_ShowName_C" null (`self.NameView`)))
  (`WidgetComponent.SetWidget` (`self.NameUi`) _returnvalue)
  (bind _returnvalue_2 (`|CreateWidget` "/Game/UI/WBP_ShowCash.WBP_ShowCash_C"))
  (bind _output_get (set `self.CashUIWid` _returnvalue_2))
  (`WidgetComponent.SetWidget` (`self.CashUI`) _output_get))

(event `CustomEvent`
  (params (cash :type Integer))
  (bind _cashuiwid (`self.CashUIWid`))
  (if (> cash 0)
    (set `/Game/UI/WBP_ShowCash.ColorCur` (make `SlateColor` (struct :`R` 0.078705 :`G` 1.0 :`A` 1.0)) _cashuiwid)
    (else
      (set `/Game/UI/WBP_ShowCash.ColorCur` (make `SlateColor` (struct :`R` 1.0 :`G` 0.059259 :`A` 1.0)) _cashuiwid)))
  (set `/Game/UI/WBP_ShowCash.CashCur` (+ cash (`/Game/UI/WBP_ShowCash.CashCur` _cashuiwid)) _cashuiwid))

(fn `GetName`
  (returns (Name :type Text))
  (return ""))

(fn `UserConstructionScript`)