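; Day-night cycle manager that runs an accelerated game clock, turns the sun and updates the sky sphere.
; Each tick it accumulates elapsed time from a configurable start time and derives sun pitch and day, hour and minute from the day fraction.
; It displays the time on a spawned clock widget and toggles the player camera pawn's light at night.
; The HUD reference is set to None, leaving its time update inactive.
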(event `self.ReceiveBeginPlay`
  (`|ExecutionSequence`
    (:`then_0`
      (`self.Get Sun and Sky`))
    (:`then_1`
      (`self.SetElapsedTimeBasedOnStartTime`))
    (:`then_2`
      (`self.SetHudRef`))
    (:`then_3`
      (bind _returnvalue (`|CreateWidget` "/Game/UI/Widgets/WBP_Clock2.WBP_Clock2_C"))
      (set `self.ClockWidgetREF` _returnvalue)
      (`UserWidget.AddToViewport` _returnvalue 0))))

(event `self.ReceiveTick`
  (params (DeltaSeconds :type "Float (single-precision)"))
  (bind (_currenttime_days _currenttime_hours _currenttime_minutes) (break `/Game/VFX/Time/Structs/Ftime` (`self.CurrentTime`)))
  (`|ExecutionSequence`
    (:`then_0`
      (`self.UpdateElapsedTime`))
    (:`then_1`
      (`self.UpdateSunPosition`))
    (:`then_2`
      (`self.UpdateCurrentTime`))
    (:`then_3`
      (set `/Game/UI/Widgets/WBP_Clock2.KTime` (`|FormatText` "Day {Days}, {Hours}:{Minutes}" _currenttime_days (`KismetTextLibrary.Conv_IntToText` _currenttime_hours false true 2 2) (`KismetTextLibrary.Conv_IntToText` _currenttime_minutes false true 2 2)) (stale `self.ReceiveBeginPlay` _returnvalue)))
    (:`then_4`
      (`self.DetermineIfNight`))))

(fn `DetermineCurrentTime`
  (returns (Time :type "/Game/VFX/Time/Structs/Ftime Structure"))
  (bind _returnvalue (`self.GetFractionOfDay`))
  (return (make `/Game/VFX/Time/Structs/Ftime` (`KismetMathLibrary.FTrunc` _returnvalue) (`KismetMathLibrary.FTrunc` (* (mod _returnvalue 1.0) 24.0)) (`KismetMathLibrary.FTrunc` (mod (* _returnvalue 1440.0) 60.0)))))

(fn `DetermineIfNight`
  (returns (ReturnValue :type Boolean))
  (bind (_currenttime_days _currenttime_hours) (break `/Game/VFX/Time/Structs/Ftime` (`self.CurrentTime`)))
  (bind _output_get (set `self.IsNight` (or (>= _currenttime_hours (`self.SunDownTime`)) (< _currenttime_hours (`self.SunUpTime`)))))
  (bind _ascamera_bp (cast `/Game/Camera/Camera_Bp` (`GameplayStatics.GetPlayerPawn` 0)))
  (if _output_get
    (`/Game/Camera/Camera_Bp.LightOn` _ascamera_bp)
    (else
      (`/Game/Camera/Camera_Bp.LightOff` _ascamera_bp)))
  (return _output_get))

(fn `Get Sun and Sky`
  (`/Engine/EditorBlueprintResources/StandardMacros.IsValid` (`self.Sun`)
    (:`Is Valid`
      _)
    (:`Is Not Valid`
      (bind _outactors (`GameplayStatics.GetAllActorsOfClass` "/Script/Engine.DirectionalLight"))
      (set `self.Sun` (`|GetArrayItem` _outactors))))
  (`/Engine/EditorBlueprintResources/StandardMacros.IsValid` (`self.Sky`)
    (:`Is Not Valid`
      (bind _outactors_2 (`GameplayStatics.GetAllActorsOfClass` "/Engine/EngineSky/BP_Sky_Sphere.BP_Sky_Sphere_C"))
      (set `self.Sky` (`|GetArrayItem` _outactors_2)))))

(fn `GetFractionOfDay`
  (returns (ReturnValue :type "Float (double-precision)"))
  (return (/ (`self.ElapsedTime`) (`self.SecondsPerDay_0`))))

(fn `GetTimeAsSeconds`
  (params (Time :type "/Game/VFX/Time/Structs/Ftime Structure (by ref)"))
  (returns (ReturnValue :type Integer))
  (bind (_days _hours _minutes) (break `/Game/VFX/Time/Structs/Ftime` Time))
  (return (+ (* _days 86400) (* _hours 3600) (* _minutes 60))))

(fn `SetElapsedTimeBasedOnStartTime`
  (set `self.ElapsedTime` (* (`self.GetTimeAsSeconds` (`self.StartTime`)) (/ (`self.SecondsPerDay_0`) 86400.0))))

(fn `SetHudRef`
  (bind _asaegame_mode_base_bp (cast `/Game/GameModeBase/AEGameModeBase_BP` (`GameplayStatics.GetGameMode`)))
  (set `self.Widget Ref2` null))

(fn `UpdateCurrentTime`
  (bind _widget_ref2 (`self.Widget Ref2`))
  (bind _output_get (set `self.CurrentTime` (`self.DetermineCurrentTime`)))
  (`/Engine/EditorBlueprintResources/StandardMacros.IsValid` _widget_ref2
    (:`Is Valid`
      (`/Game/UI/Widgets/WBP_Clock2.Set Time` _widget_ref2 _output_get (`self.ClockType`)))))

(fn `UpdateElapsedTime`
  (set `self.ElapsedTime` (+ (`self.ElapsedTime`) (`GameplayStatics.GetWorldDeltaSeconds`))))

(fn `UpdateSunPosition`
  (`SceneComponent.K2_SetRelativeRotation` (`Light.LightComponent` (`self.Sun`)) (`KismetMathLibrary.MakeRotator` 0.0 (+ (* (`self.GetFractionOfDay`) -360.0) 90.0) 30.0) false false)
  (`/Engine/EngineSky/BP_Sky_Sphere.UpdateSunDirection` (`self.Sky`)))

(fn `UserConstructionScript`
  (set `self.SecondsPerDay_0` (* (`self.MinutesPerDay`) 60.0)))