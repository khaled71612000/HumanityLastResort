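; Player camera pawn for a building-placement game that creates the HUD and glides its spring arm in from an offset at start.
; Input drives interpolated, clamped zoom, held rotation and right-drag panning, whose flag keeps the context menu from opening after a drag.
; Context clicks open a HUD menu for the Placeable under the cursor, while a camera-forward trace names objects through an interface.
; LightOn and LightOff events switch spotlights on all Buildings.
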(event `self.ReceiveBeginPlay`
  (bind _springarm (`self.SpringArm`))
  (bind _worldloc (`self.worldLoc`))
  ;[1 1 1] Add Spawn Bar
  (set `self.targetArm` (`SpringArmComponent.TargetArmLength` _springarm))
  (set `self.worldLoc` (`SceneComponent.K2_GetComponentLocation` _springarm))
  (bind _returnvalue (`|CreateWidget` "/Game/UI/HUD.HUD_C"))
  (bind _output_get (set `self.GameManagerHudREF` _returnvalue))
  (`UserWidget.AddToViewport` _output_get 0)
  (bind (_direction _fade) (`Timeline|fade`)
    (:`Update`
      (`SceneComponent.K2_SetWorldLocation` (`self.SpringArm`) (`KismetMathLibrary.VLerp` (+ _worldloc 4000.0) _worldloc _fade) false false))))

(event `GetObjectName`
  (bind _cameracomp (`self.CameraComp`))
  (bind _gamemanagerhudref (`self.GameManagerHudREF`))
  (bind _returnvalue (`SceneComponent.K2_GetComponentLocation` _cameracomp))
  ;[1 1 1] Update Name on Look
  (bind (_outhit _returnvalue_2) (`KismetSystemLibrary.LineTraceSingle` _returnvalue (+ _returnvalue (* (`SceneComponent.GetForwardVector` _cameracomp) 5000.0)) "TraceTypeQuery1"))
  (if _returnvalue_2
    (bind (_bblockinghit _binitialoverlap _time _distance _location _impactpoint _normal _impactnormal _physmat _hitactor) (`GameplayStatics.BreakHitResult` _outhit))
    (if (`KismetSystemLibrary.DoesImplementInterface` _hitactor "/Game/UI/BPI_GetNameInterFace.BPI_GetNameInterFace_C")
      (bind _name (message `/Game/UI/BPI_GetNameInterFace.GetName` _hitactor))
      (set `/Game/UI/HUD.Name` _name _gamemanagerhudref)
      (else
        (set `/Game/UI/HUD.Name` "" _gamemanagerhudref)))))

(event `InputAction|ZoomIn`
  (params (Key :type "Key Structure"))
  ;[1 1 1] MoveCamera on MouseWheel
  (:`Pressed`
    (set `self.targetArm` (`KismetMathLibrary.FClamp` (+ (`SpringArmComponent.TargetArmLength` (`self.SpringArm`)) -1500.0) 2500.0 12000.0))))

(event `self.ReceiveTick`
  (params (DeltaSeconds :type "Float (single-precision)"))
  (bind _springarm (`self.SpringArm`))
  (bind _targetarm (`self.targetArm`))
  (bind _targetarmlength (`SpringArmComponent.TargetArmLength` _springarm))
  ;[1 1 1] MoveCamera on MouseWheel
  (if (> (`KismetMathLibrary.Abs` (- _targetarmlength _targetarm)) 0.01)
    (set `SpringArmComponent.TargetArmLength` (`KismetMathLibrary.FInterpTo` _targetarmlength _targetarm DeltaSeconds 10.0) _springarm)))

(event `InputAction|ZoomOut`
  (params (Key :type "Key Structure"))
  ;[1 1 1] MoveCamera on MouseWheel
  (:`Pressed`
    (set `self.targetArm` (`KismetMathLibrary.FClamp` (+ (`SpringArmComponent.TargetArmLength` (`self.SpringArm`)) 1500.0) 2500.0 12000.0))))

(event `InputAction|RotateCamera`
  (params (Key :type "Key Structure"))
  ;[1 1 1] CameraRightClickRotation
  (:`Pressed`
    (set `self.RotateCamera` true))
  (:`Released`
    (set `self.RotateCamera` false)))

(event `InputAction|Context`
  (params (Key :type "Key Structure"))
  (bind _gamemanagerhudref (`self.GameManagerHudREF`))
  (bind _contextmenuanchor (`/Game/UI/HUD.ContextMenuAnchor` (`self.GameManagerHudREF`)))
  (bind _contextmenuanchor_2 (`/Game/UI/HUD.ContextMenuAnchor` _gamemanagerhudref))
  ;[1 1 1] Toggle Context Menu when right clicking on actor
  (:`Released`
    (if (`self.Panning`)
      _
      (elif (`MenuAnchor.IsOpen` _contextmenuanchor)
        (`MenuAnchor.Close` _contextmenuanchor)
        (else
          (bind _asplayer_controller (cast `PlayerController` (`self.GetController`)))
          (bind (_bblockinghit _binitialoverlap _time _distance _location _impactpoint _normal _impactnormal _physmat _hitactor) (`GameplayStatics.BreakHitResult` (`PlayerController.GetHitResultUnderCursorForObjects` _asplayer_controller (`|MakeArray` "ObjectTypeQuery2" :!type "EObjectTypeQuery Enum") true)))
          (if _bblockinghit
            (`/Engine/EditorBlueprintResources/StandardMacros.IsValid` _hitactor
              (:`Is Valid`
                (bind _asplaceable (cast `Placeable` _hitactor))
                (bind _returnvalue (`WidgetLayoutLibrary.GetMousePositionOnViewport`))
                (`CanvasPanelSlot.SetPosition` (`WidgetLayoutLibrary.SlotAsCanvasSlot` _contextmenuanchor_2) _returnvalue)
                (set `/Game/UI/HUD.BuildingREF` _asplaceable _gamemanagerhudref)
                (`MenuAnchor.Open` _contextmenuanchor_2 false)))))))))

(event `InputAction|UpdateName`
  (params (Key :type "Key Structure"))
  ;[1 1 1] UI Update Name
  (:`Pressed`
    (`self.GetObjectName`)))

(event `InputAxis|MouseX`
  (params (AxisValue :type "Float (single-precision)"))
  (bind _cameracomp (`self.CameraComp`))
  (bind (_returnvalue_x _returnvalue_y) (`KismetMathLibrary.BreakVector` (`SceneComponent.GetForwardVector` _cameracomp)))
  (bind (_returnvalue_x_2 _returnvalue_y_2) (`KismetMathLibrary.BreakVector` (`SceneComponent.GetRightVector` _cameracomp)))
  ;[1 1 1] CameraRightClickRotation
  (`|ExecutionSequence`
    (:`then_0`
      (if (`self.RotateCamera`)
        (`SceneComponent.K2_AddRelativeRotation` (`self.SpringArm`) (`KismetMathLibrary.MakeRotator` 0.0 (stale `InputAxis|MouseY` AxisValue) AxisValue) false false :!label _label)))
    (:`then_1`
      (if (and (!= AxisValue 0.0) (!= (stale `InputAxis|MouseY` AxisValue) 0.0) (`self.PressedRight`)) :!label _label_2
        (set `self.Panning` true)))
    (:`then_2`
      ;[1 1 1] CameraRightClickRotation
      (if (`self.Panning`)
        (`self.K2_AddActorWorldTransform` (`KismetMathLibrary.MakeTransform` (+ (* (`KismetMathLibrary.Normal` (`KismetMathLibrary.MakeVector` _returnvalue_x_2 _returnvalue_y_2)) (* AxisValue -50.0)) (* (`KismetMathLibrary.Normal` (`KismetMathLibrary.MakeVector` _returnvalue_x _returnvalue_y)) (* (stale `InputAxis|MouseY` AxisValue) -50.0)))) :!label _label_3)))))

(event `InputAxis|MouseY`
  (params (AxisValue :type "Float (single-precision)"))
  ;[1 1 1] CameraRightClickRotation
  (`|ExecutionSequence`
    (:`then_0`
      (if (`self.RotateCamera`)
        (goto _label)))
    (:`then_1`
      (goto _label_2))
    (:`then_2`
      ;[1 1 1] CameraRightClickRotation
      (if (`self.Panning`)
        (goto _label_3)))))

(event `InputAction|MouseRightClick`
  (params (Key :type "Key Structure"))
  ;[1 1 1] CameraRightClickRotation
  (:`Pressed`
    (set `self.PressedRight` true))
  (:`Released`
    (set `self.PressedRight` false)
    (`KismetSystemLibrary.Delay` 0.1)
    (set `self.Panning` false)))

(event `LightOn`
  ;[1 1 1] Lights
  (bind _outactors (`GameplayStatics.GetAllActorsOfClass` "/Script/HumanityLastResort.Building"))
  (for _array_element _outactors
    (for _array_element_2 (`self.K2_GetComponentsByClass` _array_element "/Script/Engine.SpotLightComponent")
      (`LightComponent.SetIntensity` _array_element_2 100000.0))))

(event `LightOff`
  ;[1 1 1] Lights
  (bind _outactors (`GameplayStatics.GetAllActorsOfClass` "/Script/HumanityLastResort.Building"))
  (for _array_element _outactors
    (for _array_element_2 (`self.K2_GetComponentsByClass` _array_element "/Script/Engine.SpotLightComponent")
      (`LightComponent.SetIntensity` _array_element_2 0.0))))

(fn `UserConstructionScript`)