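; Game mode that acts as the spawner for a tile-based building game, placing splines, roads and buildings on cells.
; Spawn events look up actor classes by row name in structure and building data tables.
; Buildings simulate physics, shift by a fixed or bounds-based offset, then become static after a delay.
; It also shows a clock widget, destroys buildings, and has a lock toggle whose branches both pass false.
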(event `SpawnSplineOnTile`
  (params (Location :type "Vector Structure") (RowName :type Name))
  (bind _returnvalue (`|GetDataTableRow` (`self.StructureDataBank`) RowName)
    (:`then`
      (bind _returnvalue_2 (`|SpawnActorFromClass` (`.StructureClassREF` (break `GridSplineBank` _returnvalue)) (`KismetMathLibrary.Conv_VectorToTransform` Location) "Undefined" "OverrideRootScale" null null))
      (`PrimitiveComponent.SetSimulatePhysics` (`GridSpline.SplineComponent` _returnvalue_2) true))
    (:`RowNotFound`
      (`KismetSystemLibrary.PrintString` "Error not FOUND IN DATA TABLE"))))

(event `SpawnStructureonCell`
  (params (RoleName :type "Name (by ref)") (Value :type "Transform Structure"))
  ;[1 1 1] Spawn Roads
  (bind _returnvalue (`|GetDataTableRow` (`self.StructureDataBank`) RoleName)
    (:`then`
      (`|SpawnActorFromClass` (`.StructureClassREF` (break `GridSplineBank` _returnvalue)) Value "Undefined" "OverrideRootScale" self null))
    (:`RowNotFound`
      (`KismetSystemLibrary.PrintString` "ROAD NOT IN DATATABLE"))))

(event `SpawnBuildingToCell`
  (params (Location :type "Vector Structure") (RowName :type Name))
  ;[1 1 1] **NOTE TURNED OFF SIMULATION Spawn Buildings
  (bind _returnvalue (`|GetDataTableRow` (`self.BuildDataBank`) RowName)
    (:`then`
      (bind _returnvalue_2 (`|SpawnActorFromClass` (`.BuildingsActorsClassREFF` (break `BGBuildBank` _returnvalue)) (`KismetMathLibrary.Conv_VectorToTransform` Location) "Undefined" "OverrideRootScale" null null))
      (bind _staticmeshcomponent (`Placeable.StaticMeshComponent` _returnvalue_2))
      (`PrimitiveComponent.SetSimulatePhysics` _staticmeshcomponent true)
      (if (`Placeable.isOneCell` _returnvalue_2)
        (`SceneComponent.K2_AddRelativeLocation` _staticmeshcomponent (195.0 195.0 0.0) false false)
        (else
          (bind (_min _max) (`StaticMeshComponent.GetLocalBounds` _staticmeshcomponent))
          (bind (_returnvalue_x _returnvalue_y) (`KismetMathLibrary.BreakVector` (/ (- _max _min) 2.0)))
          (`SceneComponent.K2_AddRelativeLocation` _staticmeshcomponent (`KismetMathLibrary.MakeVector` _returnvalue_x _returnvalue_y) false false)))
      (`KismetSystemLibrary.Delay` 3.0)
      (`SceneComponent.SetMobility` _staticmeshcomponent "Static"))
    (:`RowNotFound`
      (`KismetSystemLibrary.PrintString` "Error not FOUND IN DATA TABLE"))))

(event `self.ReceiveBeginPlay`
  (bind _returnvalue (`|CreateWidget` "/Game/UI/WBP_Clock.WBP_Clock_C"))
  (bind _output_get (set `self.Widget Ref` _returnvalue))
  (`UserWidget.AddToViewport` _output_get 0))

(event `LockTileServer`
  (params (BuildingREF :type "Placeable Object Reference"))
  ;[1 1 1] Lock Single Tile On Toggle
  (`/Engine/EditorBlueprintResources/StandardMacros.FlipFlop`
    (:`A`
      (`Placeable.LockPosition` BuildingREF false))
    (:`B`
      (`Placeable.LockPosition` BuildingREF false))))

(event `Destroy Building`
  (params (Building :type "Placeable Object Reference"))
  ;[1 1 1] DestroySingleTile
  (`self.K2_DestroyActor` Building))

(fn `GetGameModeREF`
  (returns (GameMode :type "/Game/GameModeBase/AEGameModeBase_BP Object Reference"))
  (return self))

(fn `UserConstructionScript`)